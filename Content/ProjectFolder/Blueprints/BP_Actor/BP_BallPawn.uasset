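; BP_BallPawn is a player pawn that rolls a ball mesh with physics torque and tracks a score.
; Movement axes apply acceleration-mode torque relative to control rotation, and look axes turn the controller.
; Holding SpaceBar raises the torque as a boost.
; IncrementScore adds to Score; the impulse jump logic is disconnected and the Hit event is empty.
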(event `Key|SpaceBar`
  (params (Key :type "Key Structure"))
  ;[1 1 1] 가속도
  (:`Pressed`
    (set `self.Torque` 10000.0))
  (:`Released`
    (set `self.Torque` 3000.0)))

(event `InputAxis|MoveForward`
  (params (AxisValue :type "Float (single-precision)"))
  ;[1 1 1] 앞뒤 이동
  (`PrimitiveComponent.AddTorqueInDegrees` (`self.BallMesh`) (* (* (`KismetMathLibrary.GetRightVector` (`self.GetControlRotation`)) (`self.Torque`)) AxisValue) "None" true))

(event `InputAxis|MoveRight`
  (params (AxisValue :type "Float (single-precision)"))
  ;[1 1 1] 좌우 이동
  (`PrimitiveComponent.AddTorqueInDegrees` (`self.BallMesh`) (* (`KismetMathLibrary.GetForwardVector` (`KismetMathLibrary.MakeRotator` 0.0 0.0 (.yaw (`self.GetControlRotation`)))) (* (`self.Torque`) AxisValue -1.0)) "None" true))

(event `InputAction|Jump`
  (params (Key :type "Key Structure"))
  ;[1 1 1] 점프
)

(event `InputTouch`
  (params (Location :type "Vector Structure") (FingerIndex :type "ETouchIndex Enum"))
  ;[1 1 1] 점프
)

(event `InputAxis|LookUp`
  (params (AxisValue :type "Float (single-precision)"))
  (`self.AddControllerPitchInput` AxisValue))

(event `self.ReceiveHit`
  (params (MyComp :type "PrimitiveComponent Object Reference") (Other :type "Actor Object Reference") (OtherComp :type "PrimitiveComponent Object Reference") (bSelfMoved :type Boolean) (HitLocation :type "Vector Structure") (HitNormal :type "Vector Structure") (NormalImpulse :type "Vector Structure") (Hit :type "HitResult Structure (by ref)"))
  ;[1 1 1] 점프 재동작
)

(event `InputAxis|Turn`
  (params (AxisValue :type "Float (single-precision)"))
  (`self.AddControllerYawInput` AxisValue))

(fn `Increment Score`
  (params (InScore :type Integer))
  (set `self.Score` (+ InScore (`self.Score`))))

(fn `UserConstructionScript`)