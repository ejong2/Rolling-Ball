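; BP_Boomb is a bomb actor that blasts the player ball when the ball hits it.
; The static mesh's hit event casts the other actor to BP_BallPawn and ignores anything else.
; It applies a velocity-change radial impulse to the ball mesh from a point below the bomb, giving an upward push.
; The bomb then destroys itself, with a 2D explosion sound and particle effect.
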(event `self.ReceiveBeginPlay`)

(event `self.StaticMesh.OnComponentHit`
  (params (HitComponent :type "PrimitiveComponent Object Reference") (OtherActor :type "Actor Object Reference") (OtherComp :type "PrimitiveComponent Object Reference") (NormalImpulse :type "Vector Structure") (Hit :type "HitResult Structure (by ref)"))
  (bind _asbp_ball_pawn (cast `/Game/ProjectFolder/Blueprints/BP_Actor/BP_BallPawn` OtherActor))
  (`PrimitiveComponent.AddRadialImpulse` (`/Game/ProjectFolder/Blueprints/BP_Actor/BP_BallPawn.BallMesh` _asbp_ball_pawn) (`KismetMathLibrary.MakeVector` (.x (`self.K2_GetActorLocation`)) (.y (`self.K2_GetActorLocation`)) (+ (.z (`self.K2_GetActorLocation`)) -200.0)) 500.0 500.0 "RIF_Constant" true)
  (`self.K2_DestroyActor`)
  (`GameplayStatics.PlaySound2D` "/Game/StarterContent/Audio/Explosion01.Explosion01" 1.0 1.0 0.0 null null)
  (`GameplayStatics.SpawnEmitterAtLocation` "/Game/StarterContent/Particles/P_Explosion.P_Explosion" (`self.K2_GetActorLocation`)))

(fn `UserConstructionScript`)