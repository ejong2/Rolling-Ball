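; Base pickup actor that awards its Points to a BP_BallPawn overlapping its sphere, with a sound and explosion effect.
; BeginPlay hides the score widget and passes it the Points value.
; On pickup, UseNumberWidget either swaps the mesh for the animated score text or destroys the actor immediately.
; Any overlap, even by a non-ball actor, also leads to destruction after a short delay.
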(event `self.ReceiveBeginPlay`
  (bind _widget (`self.Widget`))
  (`SceneComponent.SetVisibility` _widget false false)
  (bind _aspick_up_text (cast `/Game/ProjectFolder/Blueprints/PickUpBase/PickUpText` (`WidgetComponent.GetUserWidgetObject` _widget)))
  (set `/Game/ProjectFolder/Blueprints/PickUpBase/PickUpText.ScoreValue` (`self.Points`) _aspick_up_text))

(event `self.Sphere.OnComponentBeginOverlap`
  (params (OverlappedComponent :type "PrimitiveComponent Object Reference") (OtherActor :type "Actor Object Reference") (OtherComp :type "PrimitiveComponent Object Reference") (OtherBodyIndex :type Integer) (bFromSweep :type Boolean) (SweepResult :type "HitResult Structure (by ref)"))
  (`self.OnPickUp` OtherActor)
  (`KismetSystemLibrary.Delay` 0.75)
  (`self.K2_DestroyActor`))

(fn `OnPickUp`
  (params (OnActor :type "Actor Object Reference"))
  (bind _asbp_ball_pawn (cast `/Game/ProjectFolder/Blueprints/BP_BallPawn` OnActor))
  (`/Game/ProjectFolder/Blueprints/BP_BallPawn.Increment Score` _asbp_ball_pawn (`self.Points`))
  (`GameplayStatics.PlaySound2D` "/Engine/VREditor/Sounds/UI/Object_PickUp.Object_PickUp" 1.0 1.0 0.0 null null)
  (`GameplayStatics.SpawnEmitterAtLocation` "/Game/StarterContent/Particles/P_Explosion.P_Explosion" (`self.K2_GetActorLocation`))
  (if (`self.UseNumberWidget`)
    (`SceneComponent.SetVisibility` (`self.Widget`) true false)
    (`SceneComponent.SetVisibility` (`self.StaticMesh`) false false)
    (bind _aspick_up_text (cast `/Game/ProjectFolder/Blueprints/PickUpBase/PickUpText` (`WidgetComponent.GetUserWidgetObject` (`self.Widget`))))
    (`UserWidget.PlayAnimation` _aspick_up_text (`/Game/ProjectFolder/Blueprints/PickUpBase/PickUpText.NewAnimation` _aspick_up_text) 0.0 1 "Forward" 2.0 false)
    (else
      (`self.K2_DestroyActor`))))

(fn `UserConstructionScript`)